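; Creep entity Blueprint that shows its gold and experience bounty on an attached stats widget.
; Every tick it casts the widget component's user widget to StatsWidget and passes it to a display function.
; That function reads the creep's gold and experience worth and writes them to the widget as text.
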(event `self.ReceiveBeginPlay`)

(event `self.ReceiveActorBeginOverlap`
  (params (OtherActor :type "Actor Object Reference")))

(event `self.ReceiveTick`
  (params (DeltaSeconds :type "Float (single-precision)"))
  (bind _asstats_widget (cast `/Game/GameContent/UMG/StatsWidget` (`WidgetComponent.GetUserWidgetObject` (`self.Stats Widget`))))
  (bind _returnvalue (`self.getGoldWorth`))
  (set `/Game/GameContent/UMG/StatsWidget.GoldWorth` (`KismetTextLibrary.Conv_IntToText` _returnvalue) _asstats_widget)
  (bind _returnvalue_2 (`self.getExpWorth`))
  (set `/Game/GameContent/UMG/StatsWidget.ExpWorth` (`KismetTextLibrary.Conv_IntToText` _returnvalue_2) _asstats_widget))

(fn `UserConstructionScript`)