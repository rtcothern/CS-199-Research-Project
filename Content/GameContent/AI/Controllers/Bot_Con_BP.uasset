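; Bot_Con_BP is an AI controller for Bot_BP pawns that triggers their planned actions and runs attack behavior.
; It enables input from player controller 0, so pressing PlanAction makes the controlled bot execute its next action.
; RunAttackBehavior prints the target, stores it as AttackTarget in the Bot_Attack_BB blackboard, and starts the AttackBehavior tree.
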(event `self.ReceiveBeginPlay`
  (`self.EnableInput` (`GameplayStatics.GetPlayerController` 0)))

(event `InputAction|PlanAction`
  (:`Pressed`
    (bind _asbot_bp (cast `/Game/GameContent/AI/Bot_BP` (`self.K2_GetPawn`)))
    (`Bot.executeNextAction` _asbot_bp)))

(fn `RunAttackBehavior`
  (params (`Attack Target` :type "Unit Object Reference"))
  (`KismetSystemLibrary.PrintString` (`KismetStringLibrary.Conv_ObjectToString` `Attack Target`))
  (bind _blackboardcomponent (`self.UseBlackboard` "/Game/GameContent/AI/Trees/Bot_Attack_BB.Bot_Attack_BB"))
  (`BlackboardComponent.SetValueAsObject` _blackboardcomponent "AttackTarget" `Attack Target`)
  (`self.RunBehaviorTree` (`self.AttackBehavior`)))

(fn `UserConstructionScript`)