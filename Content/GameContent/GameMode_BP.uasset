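; Game mode for a two-team bot match where players start at the spectator start.
; BeginPlay creates the HUD and derives FieldWidth from a Floor-tagged brush's scale, while Tick copies team gold and average level from GameState_BP to the HUD.
; ChoosePlayerStart caches the tagged team and spectator starts.
; SpawnBots places half the bots per team in rows along X around their start, assigning IDs and spawn points.
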(event `self.ReceiveBeginPlay`
  (bind _returnvalue (`|CreateWidget` "/Game/GameContent/UMG/GameHudWidget.GameHudWidget_C"))
  (bind _output_get (set `self.HudWidget` _returnvalue))
  (`UserWidget.AddToViewport` _output_get 0)
  (bind _outactors (`GameplayStatics.GetAllActorsOfClass` "/Script/Engine.Brush"))
  (for _array_element _outactors
    (if (`self.ActorHasTag` _array_element "Floor")
      (set `self.fieldWidth` (`KismetMathLibrary.FTrunc` (* 2 (* (.y (`SceneComponent.K2_GetComponentScale` (`Brush.BrushComponent` _array_element))) 100.0))))
      (break))))

(event `self.ReceiveTick`
  (params (DeltaSeconds :type "Float (single-precision)"))
  (bind _hudwidget (`self.HudWidget`))
  (`|ExecutionSequence`
    (:`then_0`
      (bind _asgame_state_bp (cast `/Game/GameContent/GameState_BP` (`GameplayStatics.GetGameState`)))
      (`self.updateGameAttributes` (`/Game/GameContent/GameState_BP.Team_1_Gold` _asgame_state_bp) (`/Game/GameContent/GameState_BP.Team_2_Gold` _asgame_state_bp) (`/Game/GameContent/GameState_BP.Avg Level` _asgame_state_bp)))
    (:`then_1`
      (set `/Game/GameContent/UMG/GameHudWidget.TG1` (`KismetTextLibrary.Conv_IntToText` (`self.Team_1_Gold`)) _hudwidget)
      (set `/Game/GameContent/UMG/GameHudWidget.TG2` (`KismetTextLibrary.Conv_IntToText` (`self.Team_2_Gold`)) _hudwidget)
      (set `/Game/GameContent/UMG/GameHudWidget.Avg Level` (`KismetTextLibrary.Conv_IntToText` (`self.avgLevel`)) _hudwidget))))

(fn `ChoosePlayerStart`
  (params (Player :type "Controller Object Reference"))
  (returns (ReturnValue :type "Actor Object Reference"))
  (bind _outactors (`GameplayStatics.GetAllActorsOfClass` "/Script/Engine.PlayerStart"))
  (for _array_element _outactors
    (switch `name` (`PlayerStart.PlayerStartTag` _array_element)
      (:`Team 1`
        (set `self.Team 1 Start` _array_element))
      (:`Team 2`
        (set `self.Team 2 Start` _array_element))
      (:`Spectator`
        (set `self.Spectator Start` _array_element))))
  (return (`self.Spectator Start`)))

(fn `SpawnBots`
  (bind _returnvalue (/ (`self.NumberBots`) 2))
  (bind _returnvalue_2 (/ (`self.NumberBots`) 2))
  (for _index (range _returnvalue)
    (bind _returnvalue_3 (`AIBlueprintHelperLibrary.SpawnAIFromClass` "/Game/GameContent/AI/Bot_BP_Team1.Bot_BP_Team1_C" null (+ (`self.K2_GetActorLocation` (`self.Team 1 Start`)) (`KismetMathLibrary.MakeVector` (* 150 (`KismetMathLibrary.Conv_IntToDouble` (- (/ _returnvalue 2) _index))))) (struct) true))
    (bind _asbot_bp (cast `/Game/GameContent/AI/Bot_BP` _returnvalue_3))
    (set `/Game/GameContent/AI/Bot_BP.BotID` (`KismetTextLibrary.Conv_IntToText` _index) _asbot_bp)
    (set `/Game/GameContent/AI/Bot_BP.Spawn` (`self.Team 1 Start`) _asbot_bp))
  (for _index_2 (range _returnvalue_2)
    (bind _returnvalue_4 (`AIBlueprintHelperLibrary.SpawnAIFromClass` "/Game/GameContent/AI/Bot_BP_Team2.Bot_BP_Team2_C" null (+ (`KismetMathLibrary.MakeVector` (* 200 (`KismetMathLibrary.Conv_IntToDouble` (- (/ _returnvalue_2 2) _index_2)))) (`self.K2_GetActorLocation` (`self.Team 2 Start`)))))
    (bind _asbot_bp_2 (cast `/Game/GameContent/AI/Bot_BP` _returnvalue_4))
    (set `/Game/GameContent/AI/Bot_BP.BotID` (`KismetTextLibrary.Conv_IntToText` (+ _index_2 _returnvalue_2)) _asbot_bp_2)
    (set `/Game/GameContent/AI/Bot_BP.Spawn` (`self.Team 2 Start`) _asbot_bp_2))
  (return))

(fn `UserConstructionScript`)