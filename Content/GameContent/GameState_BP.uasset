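; GameState_BP is the game state that tracks match-wide team gold totals and the average player level.
; Every Tick, it resets the totals and walks PlayerArray, reading each PlayerState_BP's CurrentLevel and GoldEarned.
; Gold is added to Team 1 or Team 2 by the team of the state's BotPlayer, only when that reference is valid.
; The summed levels are divided by the PlayerArray length to give AvgLevel.
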(event `self.ReceiveBeginPlay`)

(event `self.ReceiveTick`
  (params (DeltaSeconds :type "Float (single-precision)"))
  (bind _playerarray (`self.PlayerArray`))
  (set `self.Team_1_Gold` 0)
  (set `self.Team_2_Gold` 0)
  (set `self.LevelSum` 0)
  (for _array_element _playerarray
    (bind _asplayer_state_bp (cast `/Game/GameContent/PlayerState_BP` _array_element))
    (set `self.LevelSum` (+ (`self.LevelSum`) (`/Game/GameContent/PlayerState_BP.Current_Level` _asplayer_state_bp)))
    (bind _botplayer (`/Game/GameContent/PlayerState_BP.BotPlayer` _asplayer_state_bp))
    (if (`KismetSystemLibrary.IsValid` _botplayer)
      (switch `ETeam_Enum` (`Unit.team` _botplayer)
        (:`team1`
          (set `self.Team_1_Gold` (+ (`/Game/GameContent/PlayerState_BP.Gold_Earned` _asplayer_state_bp) (`self.Team_1_Gold`))))
        (:`team2`
          (set `self.Team_2_Gold` (+ (`/Game/GameContent/PlayerState_BP.Gold_Earned` _asplayer_state_bp) (`self.Team_2_Gold`)))))))
  (set `self.Avg Level` (/ (`self.LevelSum`) (`KismetArrayLibrary.Array_Length` _playerarray))))

(fn `UserConstructionScript`)